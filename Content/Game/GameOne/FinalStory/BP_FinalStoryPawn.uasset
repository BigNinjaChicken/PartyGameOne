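; Pawn for GameOne's final story screen that shows the top game prompt as an assembled story.
; DisplayBestGamePrompt creates WBP_TopStory and fills its fragment list with prompt sentences and player responses, each response paired with its author's name.
; Responses five and six are slotted in after one and two rather than at the end.
; After a fixed delay on screen, it opens LV_GameOne.
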(event `self.DisplayBestGamePrompt`
  (bind (_topgameprompt_sentencefragments _topgameprompt_fragmentoneplayerid _topgameprompt_fragmenttwoplayerid _topgameprompt_fragmentthreeplayerid _topgameprompt_fragmentfourplayerid _topgameprompt_fragmentfiveplayerid _topgameprompt_fragmentsixplayerid) (break `GamePrompt` (`self.TopGamePrompt`)))
  (bind (_sentencefragmentone _sentencefragmentoneresponce _sentencefragmenttwo _sentencefragmenttworesponce _fragonetwogrouppoints _sentencefragmentthree _sentencefragmentthreeresponce _sentencefragmentfour _sentencefragmentfourresponce _fragthreefourgrouppoints _sentencefragmentfive _sentencefragmentfiveresponce _sentencefragmentsix _sentencefragmentsixresponce) (break `Encapsule` _topgameprompt_sentencefragments))
  (bind _returnvalue (`|CreateWidget` "/Game/Game/GameOne/FinalStory/WBP_TopStory.WBP_TopStory_C"))
  (bind _output_get (set `self.WBP_TopStory` _returnvalue))
  (bind _returnvalue_2 (`self.GetPlayerName` _topgameprompt_fragmentoneplayerid))
  (bind _returnvalue_3 (`self.GetPlayerName` _topgameprompt_fragmenttwoplayerid))
  (bind _returnvalue_4 (`self.GetPlayerName` _topgameprompt_fragmentthreeplayerid))
  (bind _returnvalue_5 (`self.GetPlayerName` _topgameprompt_fragmentfourplayerid))
  (bind _returnvalue_6 (`self.GetPlayerName` _topgameprompt_fragmentfiveplayerid))
  (bind _returnvalue_7 (`self.GetPlayerName` _topgameprompt_fragmentsixplayerid))
  (bind _allstoryfragments (`/Game/Game/GameOne/FinalStory/WBP_TopStory.AllStoryFragments` _output_get))
  (`KismetArrayLibrary.Array_Add` _allstoryfragments (make `/Game/Game/GameOne/FinalStory/S_TopStory` _sentencefragmentone))
  (`KismetArrayLibrary.Array_Add` _allstoryfragments (make `/Game/Game/GameOne/FinalStory/S_TopStory` _sentencefragmentoneresponce _returnvalue_2))
  (`KismetArrayLibrary.Array_Add` _allstoryfragments (make `/Game/Game/GameOne/FinalStory/S_TopStory` _sentencefragmentfiveresponce _returnvalue_6))
  (`KismetArrayLibrary.Array_Add` _allstoryfragments (make `/Game/Game/GameOne/FinalStory/S_TopStory` _sentencefragmenttwo))
  (`KismetArrayLibrary.Array_Add` _allstoryfragments (make `/Game/Game/GameOne/FinalStory/S_TopStory` _sentencefragmenttworesponce _returnvalue_3))
  (`KismetArrayLibrary.Array_Add` _allstoryfragments (make `/Game/Game/GameOne/FinalStory/S_TopStory` _sentencefragmentsixresponce _returnvalue_7))
  (`KismetArrayLibrary.Array_Add` _allstoryfragments (make `/Game/Game/GameOne/FinalStory/S_TopStory` _sentencefragmentthree))
  (`KismetArrayLibrary.Array_Add` _allstoryfragments (make `/Game/Game/GameOne/FinalStory/S_TopStory` _sentencefragmentthreeresponce _returnvalue_4))
  (`KismetArrayLibrary.Array_Add` _allstoryfragments (make `/Game/Game/GameOne/FinalStory/S_TopStory` _sentencefragmentfour))
  (`KismetArrayLibrary.Array_Add` _allstoryfragments (make `/Game/Game/GameOne/FinalStory/S_TopStory` _sentencefragmentfourresponce _returnvalue_5))
  (`UserWidget.AddToViewport` (`self.WBP_TopStory`) 0)
  (`KismetSystemLibrary.Delay` 15.0)
  (`GameplayStatics.OpenLevelBySoftObjectPtr` "/Game/Game/GameOne/Levels/LV_GameOne.LV_GameOne"))

(fn `UserConstructionScript`)