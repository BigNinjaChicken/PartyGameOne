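; BP_FakePlayer is a stand-in player for the start screen, with a name label and the ability to show chat messages.
; On BeginPlay it passes its PlayerName to the WBP_PlayerNameFakePlayer widget in its widget component.
; CreateChat spawns a BP_TextBox actor above itself and writes the message into that actor's WBP_ChatMessage widget.
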(event `self.ReceiveBeginPlay`
  (bind _aswbp_player_name_fake_player (cast `/Game/Game/GameOne/StartScreen/WBP_PlayerNameFakePlayer` (`WidgetComponent.GetWidget` (`self.Widget`))))
  (set `/Game/Game/GameOne/StartScreen/WBP_PlayerNameFakePlayer.PlayerName` (`self.Player Name`) _aswbp_player_name_fake_player))

(event `CreateChat`
  (params (ChatMessage :type String))
  (bind _returnvalue (`self.GetTransform`))
  (bind _returnvalue_2 (`|SpawnActorFromClass` "/Game/Game/GameOne/StartScreen/BP_TextBox.BP_TextBox_C" (`KismetMathLibrary.MakeTransform` (`KismetMathLibrary.MakeVector` (.x (.location _returnvalue)) (.y (.location _returnvalue)) (+ (.z (.location _returnvalue)) 120.0)) (.rotation _returnvalue) (.scale _returnvalue)) "Undefined" "MultiplyWithRoot" null null))
  (bind _aswbp_chat_message (cast `/Game/Game/GameOne/StartScreen/WBP_ChatMessage` (`WidgetComponent.GetWidget` (`/Game/Game/GameOne/StartScreen/BP_TextBox.Widget` _returnvalue_2))))
  (set `/Game/Game/GameOne/StartScreen/WBP_ChatMessage.ChatText` (`KismetTextLibrary.Conv_StringToText` ChatMessage) _aswbp_chat_message))

(fn `UserConstructionScript`)