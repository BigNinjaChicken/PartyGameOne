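; BP_JoinGame runs the start screen, showing joined players as fake player actors and relaying their chat messages.
; On begin play it caches the BP_SpawnArea and plays the main music.
; Each join spawns a BP_FakePlayer at a random Y within that area, maps it by name for chat, and slides it along X with rolling chair audio.
; A single shared timeline drives that slide, so each new join takes it over.
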(event `self.ReceiveBeginPlay`
  (`|ExecutionSequence`
    (:`then_1`
      (bind _returnvalue (`GameplayStatics.GetActorOfClass` "/Game/Game/GameOne/StartScreen/BP_SpawnArea.BP_SpawnArea_C"))
      (set `self.SpawnArea` _returnvalue)
      (`GameplayStatics.PlaySound2D` "/Game/Game/GameOne/Audio/Music/Cue_MainMusic.Cue_MainMusic" 1.0 1.0 0.0 null null))))

(event `self.PlayerJoined`
  (params (PlayerName :type String))
  (bind _spawnarea (`self.SpawnArea`))
  (bind (_start_x _start_y _start_z) (`KismetMathLibrary.BreakVector` (`self.Start`)))
  (bind (_returnvalue_x _returnvalue_y _returnvalue_z) (`KismetMathLibrary.BreakVector` (`self.K2_GetActorLocation` _spawnarea)))
  (bind (_boxextent_x _boxextent_y) (`KismetMathLibrary.BreakVector` (`BoxComponent.BoxExtent` (`/Game/Game/GameOne/StartScreen/BP_SpawnArea.Box` _spawnarea))))
  (bind _returnvalue (`|SpawnActorFromClass` "/Game/Game/GameOne/StartScreen/BP_FakePlayer.BP_FakePlayer_C" (`KismetMathLibrary.MakeTransform` (`KismetMathLibrary.MakeVector` _returnvalue_x (+ _returnvalue_y (`KismetMathLibrary.RandomFloatInRange` (* _boxextent_y -1.0) _boxextent_y)) _returnvalue_z)) "Undefined" "MultiplyWithRoot" null (`KismetTextLibrary.Conv_StringToText` PlayerName) null))
  (`BlueprintMapLibrary.Map_Add` (`self.FakePlayerMap`) PlayerName _returnvalue)
  (set `self.FakeActor` _returnvalue)
  (`GameplayStatics.SpawnSoundAttached` "/Game/Game/GameOne/Audio/BackgroundAudio/RollingChair.RollingChair" (`/Game/Game/GameOne/StartScreen/BP_FakePlayer.StaticMesh` _returnvalue) "None" (0.0 0.0 0.0) (struct) "KeepRelativeOffset" false 1.0 1.0 0.0 null null)
  (`|ExecutionSequence`
    (:`then_0`
      (`TimelineComponent.SetPlayRate` (`self.Timeline`) 0.5)
      (set `self.Start` (`self.K2_GetActorLocation` (`self.FakeActor`)))
      (bind (_direction _newtrack_0) (`Timeline|Timeline` :!via `PlayFromStart`)
        (:`Update`
          (`self.K2_SetActorLocation` (`self.FakeActor`) (`KismetMathLibrary.VLerp` (`self.Start`) (`KismetMathLibrary.MakeVector` (+ _start_x 250.0) _start_y _start_z) _newtrack_0) false false))))))

(event `self.DisplayChatMessage`
  (params (PlayerName :type String) (ChatMessage :type String))
  (`/Game/Game/GameOne/StartScreen/BP_FakePlayer.CreateChat` (`BlueprintMapLibrary.Map_Find` (`self.FakePlayerMap`) PlayerName) ChatMessage))

(fn `UserConstructionScript`)