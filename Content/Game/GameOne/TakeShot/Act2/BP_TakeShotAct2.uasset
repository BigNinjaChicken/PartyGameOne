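; BP_TakeShotAct2 runs the second act of the TakeShot sequence, playing a dialog line and then advancing to the next level.
; On BeginPlay it starts soft background music and binds to an everyone-ready event.
; When that fires, it plays the Dialog sound and sets a timer for the dialog's duration plus an extra offset, after which it opens the next level.
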(event `self.ReceiveBeginPlay`
  (`GameplayStatics.PlaySound2D` "/Game/Game/GameOne/Music/685599__davejf__soft-music_Cue.685599__davejf__soft-music_Cue" 1.0 1.0 0.0 null null)
  (add `self.OnEveryoneReady` (delegate `OnEveryoneReady_Event`)))

(event `OnEveryoneReady_Event`
  (bind _dialog (`self.Dialog`))
  (`GameplayStatics.PlaySound2D` _dialog 2.0 1.0 0.0 null null)
  (`KismetSystemLibrary.K2_SetTimerDelegate` (delegate `End`) (+ (`SoundBase.Duration` _dialog) (`self.AdditionalTimeOffset`))))

(event `End`
  (`self.OpenNextLevel`))

(fn `UserConstructionScript`
  (`parent.UserConstructionScript`))